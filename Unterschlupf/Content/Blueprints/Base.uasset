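; Team base actor that stores a shared metal and wood stockpile for players to deposit into and withdraw from.
; Deposit and withdraw events clamp the amount to the source, then Server events move it up to the destination's max.
; After a short delay they refresh the controller's inventory UI.
; RepNotify on team totals updates the local player's game UI when teams match, and BeginPlay initializes it after a delay.
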(event `self.ReceiveBeginPlay`
  (`KismetSystemLibrary.Delay` 2.0)
  (bind _asmain_player_controller (cast `/Game/Game/Main_PlayerController` (`GameplayStatics.GetPlayerController` 0)))
  (if (== (`/Game/Game/Main_PlayerController.Team` _asmain_player_controller) (`self.Team`))
    (bind _gameuiref (`/Game/Game/Main_PlayerController.GameuiRef` _asmain_player_controller))
    (`/Game/Game/Game_UI.Update TeamMax` _gameuiref (`self.TeamMaxMetal`) (`self.TeamMaxWood`))
    (`/Game/Game/Game_UI.Update TeamMetal` _gameuiref (`self.TeamMetal`))
    (`/Game/Game/Game_UI.Update TeamWood` _gameuiref (`self.TeamWood`))))

(event `MetalDown`
  (params (Controller :type "/Game/Game/Main_PlayerController Object Reference") (Amount :type Integer))
  (bind _teammetal (`self.TeamMetal`))
  (if (> Amount _teammetal)
    (`self.Server MD` Controller _teammetal)
    (else
      (`self.Server MD` Controller Amount))))

(event `Server MD`
  (params (Controller :type "/Game/Game/Main_PlayerController Object Reference") (Amount :type Integer))
  (bind _teammetal (`self.TeamMetal`))
  (bind _metal (`/Game/Game/Main_PlayerController.Metal` Controller))
  (bind _maxmetal (`/Game/Game/Main_PlayerController.MaxMetal` Controller))
  (bind _returnvalue (+ Amount _metal))
  (if (> Amount _teammetal)
    _
    (elif (not (== _metal _maxmetal))
      (if (>= _returnvalue _maxmetal)
        (set `self.TeamMetal` (- _teammetal (- Amount (- _returnvalue _maxmetal))))
        (set `/Game/Game/Main_PlayerController.Metal` _maxmetal Controller)
        (else
          (set `/Game/Game/Main_PlayerController.Metal` _returnvalue Controller)
          (set `self.TeamMetal` (- _teammetal Amount))))
      (`KismetSystemLibrary.Delay` 1.0)
      (`/Game/Game/Main_PlayerController.Update Invui` Controller (`self.TeamMetal`) (`self.TeamWood`)))))

(event `MetalUP`
  (params (Controller :type "/Game/Game/Main_PlayerController Object Reference") (Amount :type Integer))
  (bind _metal (`/Game/Game/Main_PlayerController.Metal` Controller))
  (if (> Amount _metal)
    (`self.Server MU` Controller _metal)
    (else
      (`self.Server MU` Controller Amount))))

(event `Server MU`
  (params (Controller :type "/Game/Game/Main_PlayerController Object Reference") (Amount :type Integer))
  (bind _teammetal (`self.TeamMetal`))
  (bind _metal (`/Game/Game/Main_PlayerController.Metal` Controller))
  (bind _teammaxmetal (`self.TeamMaxMetal`))
  (bind _returnvalue (+ _teammetal Amount))
  (if (> Amount _metal)
    _
    (elif (not (== _teammetal _teammaxmetal))
      (if (>= _returnvalue _teammaxmetal)
        (set `/Game/Game/Main_PlayerController.Metal` (- _metal (- Amount (- _returnvalue _teammaxmetal))) Controller)
        (set `self.TeamMetal` _teammaxmetal)
        (else
          (set `/Game/Game/Main_PlayerController.Metal` (- _metal Amount) Controller)
          (set `self.TeamMetal` _returnvalue)))
      (`KismetSystemLibrary.Delay` 1.0)
      (`/Game/Game/Main_PlayerController.Update Invui` Controller (`self.TeamMetal`) (`self.TeamWood`)))))

(event `WoodDown`
  (params (Controller :type "/Game/Game/Main_PlayerController Object Reference") (Amount :type Integer))
  (bind _teamwood (`self.TeamWood`))
  (if (> Amount _teamwood)
    (`self.Server wood down` Controller _teamwood)
    (else
      (`self.Server wood down` Controller Amount))))

(event `Server wood down`
  (params (Controller :type "/Game/Game/Main_PlayerController Object Reference") (Amount :type Integer))
  (bind _teamwood (`self.TeamWood`))
  (bind _wood (`/Game/Game/Main_PlayerController.Wood` Controller))
  (bind _maxwood (`/Game/Game/Main_PlayerController.MaxWood` Controller))
  (bind _returnvalue (+ Amount _wood))
  (if (> Amount _teamwood)
    _
    (elif (not (== _wood _maxwood))
      (if (>= _returnvalue _maxwood)
        (set `self.TeamWood` (- _teamwood (- Amount (- _returnvalue _maxwood))))
        (set `/Game/Game/Main_PlayerController.Wood` _maxwood Controller)
        (else
          (set `/Game/Game/Main_PlayerController.Wood` _returnvalue Controller)
          (set `self.TeamWood` (- _teamwood Amount))))
      (`KismetSystemLibrary.Delay` 1.0)
      (`/Game/Game/Main_PlayerController.Update Invui` Controller (`self.TeamMetal`) (`self.TeamWood`)))))

(event `WoodUP`
  (params (Controller :type "/Game/Game/Main_PlayerController Object Reference") (Amount :type Integer))
  (bind _wood (`/Game/Game/Main_PlayerController.Wood` Controller))
  (if (> Amount _wood)
    (`self.server wood up` Controller _wood)
    (else
      (`self.server wood up` Controller Amount))))

(event `server wood up`
  (params (Controller :type "/Game/Game/Main_PlayerController Object Reference") (Amount :type Integer))
  (bind _wood (`/Game/Game/Main_PlayerController.Wood` Controller))
  (bind _teamwood (`self.TeamWood`))
  (bind _teammaxwood (`self.TeamMaxWood`))
  (bind _returnvalue (+ _teamwood Amount))
  (if (> Amount _wood)
    _
    (elif (not (== _teamwood _teammaxwood))
      (if (>= _returnvalue _teammaxwood)
        (set `/Game/Game/Main_PlayerController.Wood` (- _wood (- Amount (- _returnvalue _teammaxwood))) Controller)
        (set `self.TeamWood` _teammaxwood)
        (else
          (set `/Game/Game/Main_PlayerController.Wood` (- _wood Amount) Controller)
          (set `self.TeamWood` _returnvalue)))
      (`KismetSystemLibrary.Delay` 1.0)
      (`/Game/Game/Main_PlayerController.Update Invui` Controller (`self.TeamMetal`) (`self.TeamWood`)))))

(fn `OnRep_TeamMetal`
  (bind _asmain_player_controller (cast `/Game/Game/Main_PlayerController` (`GameplayStatics.GetPlayerController` 0)))
  (if (== (`/Game/Game/Main_PlayerController.Team` _asmain_player_controller) (`self.Team`))
    (`/Game/Game/Game_UI.Update TeamMetal` (`/Game/Game/Main_PlayerController.GameuiRef` _asmain_player_controller) (`self.TeamMetal`))))

(fn `OnRep_TeamWood`
  (bind _asmain_player_controller (cast `/Game/Game/Main_PlayerController` (`GameplayStatics.GetPlayerController` 0)))
  (if (== (`self.Team`) (`/Game/Game/Main_PlayerController.Team` _asmain_player_controller))
    (`/Game/Game/Game_UI.Update TeamWood` (`/Game/Game/Main_PlayerController.GameuiRef` _asmain_player_controller) (`self.TeamWood`))))

(fn `UserConstructionScript`)