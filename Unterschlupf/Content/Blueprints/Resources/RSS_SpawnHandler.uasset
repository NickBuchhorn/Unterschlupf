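; Server-authoritative resource spawner that keeps four map zones stocked with Wood and Metal pickups: middle, fence middle and each player's spawn areas.
; BeginPlay and SpawnResources share one refill pass that tops each zone's counter up to its cap, alternating types via FlipFlop at random reachable navmesh points.
; Spawned resources receive a handler reference and zone group.
; Counters jump to the cap even when spawns fail.
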(event `self.ReceiveBeginPlay`
  (bind _randomlocation (`NavigationSystem.K2_GetRandomReachablePointInRadius` (`self.K2_GetActorLocation` (`self.Middle`)) 1500.0))
  (bind _randomlocation_2 (`NavigationSystem.K2_GetRandomReachablePointInRadius` (`self.K2_GetActorLocation` (`self.FenceMiddle`)) 1500.0))
  (bind _randomlocation_3 (`NavigationSystem.K2_GetRandomReachablePointInRadius` (`self.K2_GetActorLocation` (`|GetArrayItem` (`self.Player2spawns`) (`KismetMathLibrary.RandomInteger` 6))) 1500.0))
  (bind _randomlocation_4 (`NavigationSystem.K2_GetRandomReachablePointInRadius` (`self.K2_GetActorLocation` (`|GetArrayItem` (`self.Player1spawns`) (`KismetMathLibrary.RandomInteger` 6))) 1500.0))
  (`/Engine/EditorBlueprintResources/ActorMacros.Switch Has Authority` :!label _label
    (:`Authority`
      (if (< (`self.MiddleCounter`) 10)
        (for _ (range (+ (`self.MiddleCounter`) 1) 11)
          (`/Engine/EditorBlueprintResources/StandardMacros.FlipFlop`
            (:`A`
              (bind _returnvalue (`|SpawnActorFromClass` "/Game/Blueprints/Resources/Wood.Wood_C" (`KismetMathLibrary.Conv_VectorToTransform` _randomlocation) "AdjustIfPossibleButDontSpawnIfColliding" "OverrideRootScale" null null))
              (`/Engine/EditorBlueprintResources/StandardMacros.IsValid` _returnvalue
                (:`Is Valid`
                  (set `/Game/Blueprints/Resources/Wood.SpawnHandler` self _returnvalue)
                  (set `/Game/Blueprints/Resources/Wood.Group` "NewEnumerator0" _returnvalue))))
            (:`B`
              (bind _returnvalue_2 (`|SpawnActorFromClass` "/Game/Blueprints/Resources/Metal.Metal_C" (`KismetMathLibrary.Conv_VectorToTransform` _randomlocation) "AdjustIfPossibleButDontSpawnIfColliding" "OverrideRootScale" null null))
              (`/Engine/EditorBlueprintResources/StandardMacros.IsValid` _returnvalue_2
                (:`Is Valid`
                  (set `/Game/Blueprints/Resources/Metal.SpawnHandler` self _returnvalue_2)
                  (set `/Game/Blueprints/Resources/Metal.Group` "NewEnumerator0" _returnvalue_2))))))
        (set `self.MiddleCounter` 10))
      (if (< (`self.FenceCounter`) 4)
        (for _ (range (+ (`self.FenceCounter`) 1) 5)
          (`/Engine/EditorBlueprintResources/StandardMacros.FlipFlop`
            (:`A`
              (bind _returnvalue_3 (`|SpawnActorFromClass` "/Game/Blueprints/Resources/Wood.Wood_C" (`KismetMathLibrary.Conv_VectorToTransform` _randomlocation_2) "AdjustIfPossibleButDontSpawnIfColliding" "OverrideRootScale" null null))
              (`/Engine/EditorBlueprintResources/StandardMacros.IsValid` _returnvalue_3
                (:`Is Valid`
                  (set `/Game/Blueprints/Resources/Wood.SpawnHandler` self _returnvalue_3)
                  (set `/Game/Blueprints/Resources/Wood.Group` "NewEnumerator1" _returnvalue_3))))
            (:`B`
              (bind _returnvalue_4 (`|SpawnActorFromClass` "/Game/Blueprints/Resources/Metal.Metal_C" (`KismetMathLibrary.Conv_VectorToTransform` _randomlocation_2) "AdjustIfPossibleButDontSpawnIfColliding" "OverrideRootScale" null null))
              (`/Engine/EditorBlueprintResources/StandardMacros.IsValid` _returnvalue_4
                (:`Is Valid`
                  (set `/Game/Blueprints/Resources/Metal.SpawnHandler` self _returnvalue_4)
                  (set `/Game/Blueprints/Resources/Metal.Group` "NewEnumerator1" _returnvalue_4))))))
        (set `self.FenceCounter` 4))
      (if (< (`self.Player1Counter`) 10)
        (for _ (range (+ (`self.Player1Counter`) 1) 11)
          (`/Engine/EditorBlueprintResources/StandardMacros.FlipFlop`
            (:`A`
              (bind _returnvalue_5 (`|SpawnActorFromClass` "/Game/Blueprints/Resources/Wood.Wood_C" (`KismetMathLibrary.Conv_VectorToTransform` _randomlocation_4) "AdjustIfPossibleButDontSpawnIfColliding" "OverrideRootScale" null null))
              (`/Engine/EditorBlueprintResources/StandardMacros.IsValid` _returnvalue_5
                (:`Is Valid`
                  (set `/Game/Blueprints/Resources/Wood.SpawnHandler` self _returnvalue_5)
                  (set `/Game/Blueprints/Resources/Wood.Group` "NewEnumerator2" _returnvalue_5))))
            (:`B`
              (bind _returnvalue_6 (`|SpawnActorFromClass` "/Game/Blueprints/Resources/Metal.Metal_C" (`KismetMathLibrary.Conv_VectorToTransform` _randomlocation_4) "AdjustIfPossibleButDontSpawnIfColliding" "OverrideRootScale" null null))
              (`/Engine/EditorBlueprintResources/StandardMacros.IsValid` _returnvalue_6
                (:`Is Valid`
                  (set `/Game/Blueprints/Resources/Metal.SpawnHandler` self _returnvalue_6)
                  (set `/Game/Blueprints/Resources/Metal.Group` "NewEnumerator2" _returnvalue_6))))))
        (set `self.Player1Counter` 10))
      (if (< (`self.Player2Counter`) 10)
        (for _ (range (+ (`self.Player2Counter`) 1) 11)
          (`/Engine/EditorBlueprintResources/StandardMacros.FlipFlop`
            (:`A`
              (bind _returnvalue_7 (`|SpawnActorFromClass` "/Game/Blueprints/Resources/Wood.Wood_C" (`KismetMathLibrary.Conv_VectorToTransform` _randomlocation_3) "AdjustIfPossibleButDontSpawnIfColliding" "OverrideRootScale" null null))
              (`/Engine/EditorBlueprintResources/StandardMacros.IsValid` _returnvalue_7
                (:`Is Valid`
                  (set `/Game/Blueprints/Resources/Wood.SpawnHandler` self _returnvalue_7)
                  (set `/Game/Blueprints/Resources/Wood.Group` "NewEnumerator3" _returnvalue_7))))
            (:`B`
              (bind _returnvalue_8 (`|SpawnActorFromClass` "/Game/Blueprints/Resources/Metal.Metal_C" (`KismetMathLibrary.Conv_VectorToTransform` _randomlocation_3) "AdjustIfPossibleButDontSpawnIfColliding" "OverrideRootScale" null null))
              (`/Engine/EditorBlueprintResources/StandardMacros.IsValid` _returnvalue_8
                (:`Is Valid`
                  (set `/Game/Blueprints/Resources/Metal.SpawnHandler` self _returnvalue_8)
                  (set `/Game/Blueprints/Resources/Metal.Group` "NewEnumerator3" _returnvalue_8))))))
        (set `self.Player2Counter` 10)))))

(event `SpawnResources`
  (goto _label))

(fn `UserConstructionScript`)