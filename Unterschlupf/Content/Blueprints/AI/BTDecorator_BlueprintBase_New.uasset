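; A Behavior Tree decorator whose AI condition check advances a waypoint index and writes the MoveTo blackboard key, returning false on every path.
; When the controlled pawn's distance to an unset target is under 500 units, it increments WaypointIndex and sets MoveTo with no object supplied.
; The index-reset branch compares zero to zero, so it never runs, and a Zombie cast is left unused.
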(fn `PerformConditionCheckAI`
  (params (OwnerController :type "AIController Object Reference") (ControlledPawn :type "Pawn Object Reference"))
  (returns (ReturnValue :type Boolean))
  (if (> 0 0)
    (set `self.WaypointIndex` 0)
    (elif (< (`Actor.GetDistanceTo` ControlledPawn null) 500.0)
      (set `self.WaypointIndex` (+ (`self.WaypointIndex`) 1))
      (else
        (return false))))
  (`BTFunctionLibrary.SetBlackboardValueAsObject` (`self.Move to`))
  (return false))