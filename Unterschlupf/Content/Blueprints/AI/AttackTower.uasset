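; Behavior tree task that makes a zombie attack its blackboard Target, presumably a tower.
; It stops movement and, if ReadytoAttack, starts the attack cooldown, then yaws the pawn toward the target.
; A short debug-drawn Visibility trace from the zombie's arrow applies its Damage to whatever actor it hits and finishes successfully.
; It fails when not ready or the target is invalid, but never finishes if the trace misses.
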(event `self.ReceiveExecuteAI`
  (params (OwnerController :type "AIController Object Reference") (ControlledPawn :type "Pawn Object Reference"))
  (bind _aszombie (cast `/Game/Blueprints/AI/Zombie` ControlledPawn :!pure true))
  (bind _arrow1 (`self.Arrow1`))
  (bind _returnvalue (`BTFunctionLibrary.GetBlackboardValueAsActor` (`self.Target`)))
  (bind _returnvalue_2 (`SceneComponent.K2_GetComponentLocation` _arrow1))
  (`|ExecutionSequence`
    (:`then_0`
      (set `self.Arrow1` (`/Game/Blueprints/AI/Zombie.Arrow1` _aszombie))
      (set `self.Damage` (`/Game/Blueprints/AI/Zombie.Damage` _aszombie))
      (`Controller.StopMovement` OwnerController))
    (:`then_1`
      (if (`/Game/Blueprints/AI/Zombie.ReadytoAttack` _aszombie)
        (`/Game/Blueprints/AI/Zombie.attackcd` _aszombie)
        (`/Engine/EditorBlueprintResources/StandardMacros.IsValid` _returnvalue
          (:`Is Valid`
            (`Actor.K2_SetActorRotation` _aszombie (`KismetMathLibrary.MakeRotator` (.roll (`Actor.K2_GetActorRotation` ControlledPawn)) (.pitch (`Actor.K2_GetActorRotation` ControlledPawn)) (.yaw (`KismetMathLibrary.FindLookAtRotation` (`Actor.K2_GetActorLocation` ControlledPawn) (`Actor.K2_GetActorLocation` _returnvalue)))) false)
            (bind (_outhit _returnvalue_3) (`KismetSystemLibrary.LineTraceSingle` _returnvalue_2 (+ (* (`SceneComponent.GetForwardVector` _arrow1) 300.0) _returnvalue_2) "TraceTypeQuery1" false (`|MakeArray` ControlledPawn :!type "Actor Object Reference") "ForDuration"))
            (if _returnvalue_3
              (bind (_bblockinghit _binitialoverlap _time _location _impactpoint _normal _impactnormal _physmat _hitactor) (`GameplayStatics.BreakHitResult` _outhit))
              (`/Engine/EditorBlueprintResources/StandardMacros.IsValid` _hitactor
                (:`Is Valid`
                  (`GameplayStatics.ApplyDamage` _hitactor (`self.Damage`) null ControlledPawn)
                  (`self.FinishExecute` true)))))
          (:`Is Not Valid`
            (`self.FinishExecute` false :!label _label)))
        (else
          (goto _label))))))