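; Main_AIController is the AI controller that starts the behavior of a Zombie pawn.
; Its StartAi event initializes the ZombieBlackBoard, sets ValidPath to true, and copies the zombie's Attacker and FollowPath flags into blackboard keys.
; It then runs the AIThree behavior tree; Tick and the construction script are empty.
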(event `StartAi`
  (bind _aszombie (cast `/Game/Blueprints/AI/Zombie` (`self.K2_GetPawn`) :!pure true))
  (bind _blackboardcomponent (`self.UseBlackboard` "/Game/Blueprints/AI/ZombieBlackBoard.ZombieBlackBoard"))
  (`BlackboardComponent.SetValueAsBool` _blackboardcomponent (`self.ValidPath`) true)
  (`BlackboardComponent.SetValueAsBool` _blackboardcomponent (`self.Attacker`) (`/Game/Blueprints/AI/Zombie.Attacker` _aszombie))
  (`BlackboardComponent.SetValueAsBool` _blackboardcomponent (`self.FollowPAth`) (`/Game/Blueprints/AI/Zombie.FollowPath` _aszombie))
  (`self.RunBehaviorTree` "/Game/Blueprints/AI/AIThree.AIThree"))

(fn `UserConstructionScript`)