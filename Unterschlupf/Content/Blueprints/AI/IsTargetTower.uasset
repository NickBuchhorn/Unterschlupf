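; Behavior tree decorator for Zombie AI that passes only when the zombie's current Target is a tower.
; It identifies towers by searching the Target's display name for the substring "tower" rather than checking its class.
; On a match it also writes the Target and its location to the blackboard as a side effect of the condition check.
; An invalid Target or non-matching name fails the check.
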(fn `PerformConditionCheckAI`
  (params (OwnerController :type "AIController Object Reference") (ControlledPawn :type "Pawn Object Reference"))
  (returns (ReturnValue :type Boolean))
  (bind _target (`/Game/Blueprints/AI/Zombie.Target` (cast `/Game/Blueprints/AI/Zombie` ControlledPawn :!pure true)))
  (`/Engine/EditorBlueprintResources/StandardMacros.IsValid` _target
    (:`Is Valid`
      (if (`KismetStringLibrary.Contains` (`KismetSystemLibrary.GetDisplayName` _target) "tower" false true)
        (`BTFunctionLibrary.SetBlackboardValueAsVector` (`self.targetlocation`) (`Actor.K2_GetActorLocation` _target))
        (`BTFunctionLibrary.SetBlackboardValueAsObject` (`self.target`) _target)
        (return true)
        (else
          _)))
    (:`Is Not Valid`
      _))
  (return false))