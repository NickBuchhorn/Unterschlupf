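; Storage building Blueprint that raises its team's metal and wood capacity.
; On UpdateBuild, the server adds StorageToAdd to the Base's team maximums and restores the cube's original material.
; AnyDamage reduces HP, and at zero or below it subtracts the same capacity from the Base and destroys the actor.
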(event `self.Update build`
  (bind _base (`self.Base`))
  (bind _storage_to_add (`self.Storage to add`))
  (`/Engine/EditorBlueprintResources/ActorMacros.Switch Has Authority`
    (:`Authority`
      (set `/Game/Blueprints/Base.TeamMaxMetal` (+ (`/Game/Blueprints/Base.TeamMaxMetal` _base) _storage_to_add) _base)
      (set `/Game/Blueprints/Base.TeamMaxWood` (+ (`/Game/Blueprints/Base.TeamMaxWood` _base) _storage_to_add) _base)
      (`PrimitiveComponent.SetMaterial` (`self.Cube`) 0 (`self.OriginalMaterial`)))))

(event `self.ReceiveAnyDamage`
  (params (Damage :type "Float (single-precision)") (DamageType :type "DamageType Object Reference") (InstigatedBy :type "Controller Object Reference") (DamageCauser :type "Actor Object Reference"))
  (bind _base (`self.Base`))
  (bind _storage_to_add (`self.Storage to add`))
  (bind _output_get (set `self.HP` (- (`self.HP`) Damage)))
  (if (<= _output_get 0.0)
    (set `/Game/Blueprints/Base.TeamMaxMetal` (- (`/Game/Blueprints/Base.TeamMaxMetal` _base) _storage_to_add) _base)
    (set `/Game/Blueprints/Base.TeamMaxWood` (- (`/Game/Blueprints/Base.TeamMaxWood` _base) _storage_to_add) _base)
    (`self.K2_DestroyActor`)))

(fn `UserConstructionScript`
  (`parent.UserConstructionScript`))