(event `Repair`
  (bind _hp (`self.HP`))
  (if (not (>= _hp (`self.MaxHP`)))
    (set `self.HP` (+ _hp (`self.Buildspeed`)))))

(event `self.ReceiveBeginPlay`
  (set `self.Buildspeed` (* (/ (`self.MaxHP`) 100) 10)))

(event `Build`
  (bind _hp (`self.HP`))
  (bind _maxhp (`self.MaxHP`))
  (set `self.HP` (+ _hp (`self.Buildspeed`)))
  (if (>= _hp _maxhp)
    (set `self.HP` _maxhp)
    (set `self.Build?` true)
    (`PrimitiveComponent.SetMaterial` (`self.Cube`) 0 (`self.OriginalMaterial`))))

(event `update new building`
  (`self.update`))

(event `update`
  (`self.SetActorEnableCollision` true)
  (`PrimitiveComponent.SetMaterial` (`self.Cube`) 0 "/Game/Materials/T_Grey_Mat.T_Grey_Mat"))

(fn `UserConstructionScript`)