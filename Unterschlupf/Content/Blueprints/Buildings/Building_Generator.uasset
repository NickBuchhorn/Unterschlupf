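; Generator building Blueprint that supplies energy to its Base for as long as it stands.
; UpdateBuild adds EnergytoAdd to the Base's Energy and MaxEnergy on the authority only, then restores the cube's original material.
; AnyDamage reduces HP and, at zero or below, subtracts that same amount from both values and destroys the actor.
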(event `self.Update build`
  (bind _base (`self.Base`))
  (bind _energytoadd (`self.EnergytoAdd`))
  (`/Engine/EditorBlueprintResources/ActorMacros.Switch Has Authority`
    (:`Authority`
      (set `/Game/Blueprints/Base.Energy` (+ (`/Game/Blueprints/Base.Energy` _base) _energytoadd) _base)
      (set `/Game/Blueprints/Base.MaxEnergy` (+ (`/Game/Blueprints/Base.MaxEnergy` _base) _energytoadd) _base))
    (:`Remote`
      _))
  (`PrimitiveComponent.SetMaterial` (`self.Cube`) 0 (`self.OriginalMaterial`)))

(event `self.ReceiveAnyDamage`
  (params (Damage :type "Float (single-precision)") (DamageType :type "DamageType Object Reference") (InstigatedBy :type "Controller Object Reference") (DamageCauser :type "Actor Object Reference"))
  (bind _energytoadd (`self.EnergytoAdd`))
  (bind _base (`self.Base`))
  (bind _output_get (set `self.HP` (- (`self.HP`) Damage)))
  (if (<= _output_get 0.0)
    (set `/Game/Blueprints/Base.Energy` (- (`/Game/Blueprints/Base.Energy` _base) _energytoadd) _base)
    (set `/Game/Blueprints/Base.MaxEnergy` (- (`/Game/Blueprints/Base.MaxEnergy` _base) _energytoadd) _base)
    (`self.K2_DestroyActor`)))

(fn `UserConstructionScript`
  (`parent.UserConstructionScript`))