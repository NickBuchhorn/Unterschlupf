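; Building gate that opens and closes when interacted with, provided its Build flag is true.
; A FlipFlop alternates between playing the Open timeline forward and in reverse, with IsMoving blocking retriggers during movement.
; The timeline moves StaticMesh2 vertically by writing its track value directly as absolute world Z, keeping X and Y unchanged.
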(event `self.Interact`
  (if (`self.Build?`)
    (`self.Open/Close`)))

(event `Open/Close`
  (bind _staticmesh2 (`self.StaticMesh2`))
  (if (not (`self.IsMoving`))
    (set `self.IsMoving` true)
    (`/Engine/EditorBlueprintResources/StandardMacros.FlipFlop`
      (:`A`
        (bind (_direction _time) (`Timeline|Open` :!via `PlayFromStart` :!label _label)
          (:`Update`
            (`SceneComponent.K2_SetWorldLocation` _staticmesh2 (`KismetMathLibrary.MakeVector` (.x (`SceneComponent.K2_GetComponentLocation` _staticmesh2)) (.y (`SceneComponent.K2_GetComponentLocation` _staticmesh2)) _time) false false))
          (:`Finished`
            (set `self.IsMoving` false))))
      (:`B`
        (goto _label :!via `ReverseFromEnd`)))))

(fn `UserConstructionScript`
  (`parent.UserConstructionScript`))