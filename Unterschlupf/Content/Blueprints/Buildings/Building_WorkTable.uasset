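; Building_WorkTable is a placeable work table building Blueprint.
; Its UpdateBuild event restores the original material on the Cube mesh, likely when construction completes.
; On the server only, it then sets the WorkTablebuild flag on its Base reference to record that the table is built.
; BeginPlay, overlap and Tick are unused stubs.
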(event `self.Update build`
  (`PrimitiveComponent.SetMaterial` (`self.Cube`) 0 (`self.OriginalMaterial`))
  (`/Engine/EditorBlueprintResources/ActorMacros.Switch Has Authority`
    (:`Authority`
      (set `/Game/Blueprints/Base.WorkTablebuild` true (`self.Base`)))))

(fn `UserConstructionScript`
  (`parent.UserConstructionScript`))