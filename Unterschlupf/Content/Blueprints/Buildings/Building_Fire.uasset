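; Fire building Blueprint that acts as a team safe zone, pausing stamina drain for friendly players near it.
; Its Regen volume finds overlapping players by name prefix and cast, stopping drain on entry and restarting it on exit for same-team players.
; UpdateBuild restores the cube's original material and enables the volume's collision.
; SetBuildSpeed derives build speed from MaxHP, with scaling that cancels out to the same value.
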(event `self.SetBuildSpeed`
  (params (Percent :type "Float (single-precision)"))
  (set `self.Buildspeed` (* (/ (`self.MaxHP`) 100.0) 100.0)))

(event `self.Regen.OnComponentBeginOverlap`
  (params (OverlappedComponent :type "PrimitiveComponent Object Reference") (OtherActor :type "Actor Object Reference") (OtherComp :type "PrimitiveComponent Object Reference") (OtherBodyIndex :type Integer) (bFromSweep :type Boolean) (SweepResult :type "HitResult Structure (by ref)"))
  (if (`KismetStringLibrary.StartsWith` (`KismetSystemLibrary.GetObjectName` OtherActor) "player")
    (bind _asplayer (cast `/Game/Game/Player` OtherActor))
    (if (== (`/Game/Game/Player.Team` _asplayer) (`self.Team`))
      (`/Game/Game/Player.stopdrain` _asplayer))))

(event `self.Regen.OnComponentEndOverlap`
  (params (OverlappedComponent :type "PrimitiveComponent Object Reference") (OtherActor :type "Actor Object Reference") (OtherComp :type "PrimitiveComponent Object Reference") (OtherBodyIndex :type Integer))
  (if (`KismetStringLibrary.StartsWith` (`KismetSystemLibrary.GetObjectName` OtherActor) "player")
    (bind _asplayer (cast `/Game/Game/Player` OtherActor))
    (if (== (`/Game/Game/Player.Team` _asplayer) (`self.Team`))
      (`/Game/Game/Player.StartStaminadrain` _asplayer))))

(event `self.Update build`
  (`PrimitiveComponent.SetMaterial` (`self.Cube`) 0 (`self.OriginalMaterial`))
  (`PrimitiveComponent.SetCollisionEnabled` (`self.Regen`) "QueryAndPhysics"))

(fn `UserConstructionScript`
  (`parent.UserConstructionScript`))