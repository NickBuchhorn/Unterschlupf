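; Tower building Blueprint that automatically damages zombies that enter its Range component.
; Once Build is set, server-side overlaps queue actors with "zombie"-prefixed names in Targets and start a looping fire timer through a DoOnce.
; Each tick of that timer aims the Arrow at the first target and applies instant damage, or drops it if invalid.
; Leaving range never removes targets, and the empty-list timer stop sits only on the valid-target branch.
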(event `self.Range.OnComponentBeginOverlap`
  (params (OverlappedComponent :type "PrimitiveComponent Object Reference") (OtherActor :type "Actor Object Reference") (OtherComp :type "PrimitiveComponent Object Reference") (OtherBodyIndex :type Integer) (bFromSweep :type Boolean) (SweepResult :type "HitResult Structure (by ref)"))
  (`KismetSystemLibrary.PrintString` "Hello")
  (if (`self.Build?`)
    (if (`KismetSystemLibrary.IsServer`)
      (if (`KismetStringLibrary.StartsWith` (`KismetSystemLibrary.GetDisplayName` OtherActor) "zombie")
        (`KismetArrayLibrary.Array_AddUnique` (`self.Targets`) OtherActor)
        (`/Engine/EditorBlueprintResources/StandardMacros.DoOnce` false :!label _label
          (:`Completed`
            (`KismetSystemLibrary.K2_SetTimer` null "fire" 1.0 true)))))))

(event `fire`
  (bind _targets (`self.Targets`))
  (bind _arrow (`self.Arrow`))
  (bind _output (`|GetArrayItem` _targets))
  (`/Engine/EditorBlueprintResources/StandardMacros.IsValid` _output
    (:`Is Valid`
      (`SceneComponent.K2_SetWorldRotation` _arrow (`KismetMathLibrary.FindLookAtRotation` (`SceneComponent.K2_GetComponentLocation` _arrow) (`self.K2_GetActorLocation` _output)) false false)
      (`GameplayStatics.ApplyDamage` _output (`self.Damage`) null self)
      (if (<= (`KismetArrayLibrary.Array_Length` _targets) 0)
        (`KismetSystemLibrary.K2_ClearTimer` null "fire")
        (goto _label :!via `Reset`)))
    (:`Is Not Valid`
      (`KismetArrayLibrary.Array_Remove` _targets))))

(fn `UserConstructionScript`
  (`parent.UserConstructionScript`))